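; Display actor that plays an animation on a skeletal mesh and shows that animation's name in an attached widget.
; The construction script passes the default animation data to SetAnimationData, which updates the mesh's animation and writes the asset's display name to the AnimationDisplay widget.
; BeginPlay writes the default animation's name to the widget again.
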(event EventBeginPlay
  (bind _asanimation_display (Utilities|Casting|CastToAnimationDisplay (UserInterface|GetWidget (Variables|Default|GetWidget))))
  (Variables|/Game/Blueprints/AnimationDisplay/AnimationDisplay.AnimationDisplay_C|SetTextValue _asanimation_display (Utilities|Text|ToText(String) (Utilities|GetDisplayName (.animtoplay (Variables|Default|GetDefaultAnimation%20Data))))))

(fn ConstructionScript
  (CallFunction|SetAnimationData (Variables|Default|GetDefaultAnimation%20Data)))

(fn SetAnimationData
  (params (Animation%20Data :type Single%20Animation%20Play%20Data%20Structure))
  (bind _output_get (Variables|/Script/Engine.SkeletalMeshComponent|SetAnimationData (Variables|Default|GetSkeletalMesh) Animation%20Data))
  (Components|Animation|SetAnimation (Variables|Default|GetSkeletalMesh) (.AnimToPlay (Utilities|Struct|BreakSingleAnimationPlayData _output_get)))
  (bind _asanimation_display (Utilities|Casting|CastToAnimationDisplay (UserInterface|GetWidget (Variables|Default|GetWidget))))
  (Variables|/Game/Blueprints/AnimationDisplay/AnimationDisplay.AnimationDisplay_C|SetTextValue _asanimation_display (Utilities|Text|ToText(String) (Utilities|GetDisplayName (.AnimToPlay (Utilities|Struct|BreakSingleAnimationPlayData _output_get))))))