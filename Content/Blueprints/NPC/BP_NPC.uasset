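; BP_NPC is an NPC Blueprint that uses the Manny materials, tinted blue.
; Its Construction Script creates dynamic material instances from MI_Manny_01 and MI_Manny_02 and stores them in Mat01 and Mat02.
; Each instance gets a hard-coded blue Tint parameter and is applied to the matching Mesh material slot.
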(fn ConstructionScript
  (Utilities|FlowControl|Sequence
    (:then_0
      (bind _returnvalue (Rendering|Material|CreateDynamicMaterialInstance "/Game/Characters/Mannequins/Materials/Instances/Manny/MI_Manny_01.MI_Manny_01" "None" "None" :!class /Script/Engine.KismetMaterialLibrary))
      (bind _output_get (LocalVariables|SetMat01 _returnvalue))
      (Rendering|Material|SetVectorParameterValue _output_get "Tint" "(R=0.000000,G=0.000000,B=1.000000,A=1.000000)" :!class /Script/Engine.MaterialInstanceDynamic)
      (Rendering|Material|SetMaterial (Variables|Character|GetMesh) 0 (LocalVariables|GetMat01)))
    (:then_1
      (bind _returnvalue_2 (Rendering|Material|CreateDynamicMaterialInstance "/Game/Characters/Mannequins/Materials/Instances/Manny/MI_Manny_02.MI_Manny_02" "None" "None" :!class /Script/Engine.KismetMaterialLibrary))
      (bind _output_get_2 (LocalVariables|SetMat02 _returnvalue_2))
      (Rendering|Material|SetVectorParameterValue _output_get_2 "Tint" "(R=0.000000,G=0.000000,B=1.000000,A=1.000000)" :!class /Script/Engine.MaterialInstanceDynamic)
      (Rendering|Material|SetMaterial (Variables|Character|GetMesh) 1 (LocalVariables|GetMat02)))))