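; Blueprint function library that converts between level and experience points for five leveling speed curves, from Slow to Fast.
; Two entry functions select a per-speed helper: required experience is level cubed times that speed's multiplier, floored.
; The reverse divides experience by the multiplier and floors an approximate cube root.
; Its truncated 0.333333 exponent can return one level low at exact thresholds.
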(fn GetExperiencePointsNeeded
  (params (Level :type Integer) (LevelingSpeed :type EnumLevelingSpeed%20Enum :default "NewEnumerator0"))
  (return (Utilities|Select :Index LevelingSpeed :NewEnumerator0 (Private|LevelToExperience|GetExpSlow Level) :NewEnumerator1 (Private|LevelToExperience|GetExpMediumSlow Level) :NewEnumerator2 (Private|LevelToExperience|GetExpMedium Level) :NewEnumerator3 (Private|LevelToExperience|GetExpMediumFast Level) :NewEnumerator4 (Private|LevelToExperience|GetExpFast Level))))

(fn GetLevelforExperiencePoints
  (params (ExperiencePoints :type Integer) (LevelingSpeed :type EnumLevelingSpeed%20Enum :default "NewEnumerator0"))
  (return (Utilities|Select :Index LevelingSpeed :NewEnumerator0 (private|ExperienceToLevel|GetLevelSlow ExperiencePoints) :NewEnumerator1 (private|ExperienceToLevel|GetLevelMediumSlow ExperiencePoints) :NewEnumerator2 (private|ExperienceToLevel|GetLevelMedium ExperiencePoints) :NewEnumerator3 (private|ExperienceToLevel|GetLevelMediumFast ExperiencePoints) :NewEnumerator4 (private|ExperienceToLevel|GetLevelFast ExperiencePoints))))

(fn GetLevelSlow
  (params (ExperiencePoints :type Integer))
  (return (Math|Float|Floor (Math|Float|Power (/ ExperiencePoints (/ 5.0 4.0)) 0.333333))))

(fn GetLevelMediumSlow
  (params (ExperiencePoints :type Integer))
  (return (Math|Float|Floor (Math|Float|Power (/ ExperiencePoints (/ 21.0 2e+01)) 0.333333))))

(fn GetLevelMedium
  (params (ExperiencePoints :type Integer))
  (return (Math|Float|Floor (Math|Float|Power (Math|Conversions|ToFloat(Integer) ExperiencePoints) 0.333333))))

(fn GetLevelMediumFast
  (params (ExperiencePoints :type Integer))
  (return (Math|Float|Floor (Math|Float|Power (/ ExperiencePoints (/ 19.0 2e+01)) 0.333333))))

(fn GetLevelFast
  (params (ExperiencePoints :type Integer))
  (return (Math|Float|Floor (Math|Float|Power (/ ExperiencePoints (/ 4.0 5.0)) 0.333333))))

(fn GetExpSlow
  (params (Level :type Integer))
  (return (Math|Float|Floor (* (Math|Float|Power (Math|Conversions|ToFloat(Integer) Level) 3.0) (/ 5.0 4.0)))))

(fn GetExpMediumSlow
  (params (Level :type Integer))
  (return (Math|Float|Floor (* (Math|Float|Power (Math|Conversions|ToFloat(Integer) Level) 3.0) (/ 21.0 2e+01)))))

(fn GetExpMedium
  (params (Level :type Integer))
  (return (Math|Float|Floor (Math|Float|Power (Math|Conversions|ToFloat(Integer) Level) 3.0))))

(fn GetExpMediumFast
  (params (Level :type Integer))
  (return (Math|Float|Floor (* (Math|Float|Power (Math|Conversions|ToFloat(Integer) Level) 3.0) (/ 19.0 2e+01)))))

(fn GetExpFast
  (params (Level :type Integer))
  (return (Math|Float|Floor (* (Math|Float|Power (Math|Conversions|ToFloat(Integer) Level) 3.0) (/ 4.0 5.0)))))