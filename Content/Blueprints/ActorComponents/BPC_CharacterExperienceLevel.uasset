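; Character component that tracks experience points and level, exposing getters for both and for the experience still needed to level up.
; GainExperience adds points, refreshes the remaining amount, then recalculates level from total experience, firing OnLeveledUp if it rises.
; Thresholds and levels come from helper functions scaled by LevelingSpeed.
; The remaining amount is computed before the level updates, so it targets the old level's successor.
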(fn GetCurrentLevel
  (return (Variables|Private|ExperienceLevel|GetCurrentLevel)))

(fn GetExperienceforLevelUp
  (return (Variables|private|ExperienceLevel|GetExperienceForLevelUp)))

(fn GetCurrentExperience
  (return (Variables|private|ExperienceLevel|GetCurrentExperience)))

(fn UpdateExperienceforLevelUp
  (bind _output_get (Variables|private|ExperienceLevel|SetExperienceForLevelUp (- (CallFunction|GetExperiencePointsNeeded (+ (ExperienceLevel|GetCurrentLevel) 1) (Variables|Private|ExperienceLevel|GetLevelingSpeed)) (Variables|private|ExperienceLevel|GetCurrentExperience))))
  (return _output_get))

(fn GainExperience
  (params (ExperienceGained :type Integer))
  (LocalVariables|SetOldExperiencce (Variables|private|ExperienceLevel|GetCurrentExperience))
  (LocalVariables|SetOldLevel (Variables|Private|ExperienceLevel|GetCurrentLevel))
  (Variables|private|ExperienceLevel|SetCurrentExperience (+ (LocalVariables|GetOldExperiencce) ExperienceGained))
  (Private|ExperienceLevel|UpdateExperienceforLevelUp)
  (bind _newcurrentlevel (Private|ExperienceLevel|UpdateCurrentLevel))
  (if (> _newcurrentlevel (LocalVariables|GetOldLevel))
    (Default|CallOnLeveledUp (Variables|Private|ExperienceLevel|GetCurrentLevel) (LocalVariables|GetOldLevel))))

(fn UpdateCurrentLevel
  (bind _output_get (Variables|Private|ExperienceLevel|SetCurrentLevel (CallFunction|GetLevelforExperiencePoints (Variables|private|ExperienceLevel|GetCurrentExperience) (Variables|Private|ExperienceLevel|GetLevelingSpeed))))
  (return _output_get))