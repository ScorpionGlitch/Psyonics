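; BPC_CharacterStats is an actor component that tracks a character's health through damage and healing.
; TakeDamage subtracts positive damage, clamps health between zero and MaximumHealth, and calls the OnDeath dispatcher with the damage details when health reaches zero.
; Heal adds positive amounts to CurrentHealth but clamps the result to MaximumXP rather than MaximumHealth, which looks like a bug.
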(fn TakeDamage
  (params (Damaged%20Actor :type Actor%20Object%20Reference) (Damage :type Float%20%28double-precision%29) (Damage%20Type :type Damage%20Type%20Object%20Reference) (Instigated%20By :type Controller%20Object%20Reference) (Damage%20Causer :type Actor%20Object%20Reference))
  (if (> Damage 0.0)
    (bind _output_get (Variables|Health|SetCurrentHealth (Math|Float|Clamp(Float) (- (Variables|Health|GetCurrentHealth) Damage) 0.0 (Variables|Health|GetMaximumHealth))))
    (if (<= _output_get 0.0)
      (Default|CallOnDeath Damaged%20Actor Damage Damage%20Type Instigated%20By Damage%20Causer))))

(fn Heal
  (params (HealedAmount :type Float%20%28double-precision%29))
  (if (> HealedAmount 0.0)
    (Variables|Health|SetCurrentHealth (Math|Float|Clamp(Float) (+ (Variables|Health|GetCurrentHealth) HealedAmount) 0.0 (Variables|XP|GetMaximumXP)))))