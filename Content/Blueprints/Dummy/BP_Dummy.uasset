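; Yellow-tinted dummy character that the player can stealth-assassinate through an interact action.
; An overlap area toggles the prompt for the player; Interact sets a motion-warp target on the attacker and plays paired knife montages on both characters.
; Attacker montage notifies apply stab and kill damage to the dummy.
; The health component updates the health bar and, on death, triggers a pelvis-down ragdoll and removes the controller and assassination components.
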(event OnComponentBeginOverlap(AssassinationArea)
  (params (OverlappedComponent :type Primitive%20Component%20Object%20Reference) (OtherActor :type Actor%20Object%20Reference) (OtherComp :type Primitive%20Component%20Object%20Reference) (OtherBodyIndex :type Integer) (bFromSweep :type Boolean) (SweepResult :type Hit%20Result%20Structure%20%28by%20ref%29))
  (if (== OtherActor (Game|GetPlayerCharacter 0))
    (bind _assassinateprompt (Variables|Default|GetAssassinatePrompt)
      (:then
        (Rendering|SetVisibility _assassinateprompt true false))
      (:else))))

(event OnComponentEndOverlap(AssassinationArea)
  (params (OverlappedComponent :type Primitive%20Component%20Object%20Reference) (OtherActor :type Actor%20Object%20Reference) (OtherComp :type Primitive%20Component%20Object%20Reference) (OtherBodyIndex :type Integer))
  (if (== OtherActor (Game|GetPlayerCharacter 0))
    (bind _assassinateprompt (Variables|Default|GetAssassinatePrompt)
      (:then
        (Rendering|SetVisibility _assassinateprompt false false))
      (:else))))

(event Custom|OnDeath
  (params (Damaged%20Actor :type Actor%20Object%20Reference) (Damage :type Float%20%28double-precision%29) (Damage%20Type :type Damage%20Type%20Object%20Reference) (Instigated%20By :type Controller%20Object%20Reference) (Damage%20Causer :type Actor%20Object%20Reference))
  (bind _mesh (Variables|Character|GetMesh))
  (Class|SkeletalMeshComponent|SetAllBodiesBelowSimulatePhysics (Variables|Character|GetMesh) (Utilities|Name|MakeLiteralName "pelvis") true true)
  (Collision|SetCollisionEnabled _mesh "QueryAndPhysics")
  (Collision|SetCollisionProfileName _mesh "Enemy" true :!class /Script/Engine.PrimitiveComponent)
  (Variables|/Script/Engine.PrimitiveComponent|SetCanCharacterStepUpOn _mesh "ECB_Yes")
  (Collision|SetCollisionEnabled (Variables|Default|GetCapsuleComponent) "NoCollision")
  (Actor|DestroyActor (Pawn|GetController))
  (Components|DestroyComponent (Variables|Default|GetHealthBar)))

(event Custom|OnHealthUpdated
  (params (CurrentHealth :type Float%20%28double-precision%29) (MaximumHealth :type Float%20%28double-precision%29) (HealthPercentage :type Float%20%28double-precision%29))
  (bind _healthbar (Variables|Default|GetHealthBar)
    (:then
      (Class|BPIHealthBar|SetHealthPercentage(Message) (UserInterface|GetWidget _healthbar) HealthPercentage))
    (:else)))

(event EventBeginPlay
  (bind _bpc_healthcomponent (Variables|Default|GetBPC_HealthComponent))
  (EventDispatchers|BindEventtoOnDeath _bpc_healthcomponent (delegate Custom|OnDeath))
  (EventDispatchers|AssignOnHealthUpdated _bpc_healthcomponent (delegate Custom|OnHealthUpdated))
  (Class|BPIHealthBar|SetHealthPercentage(Message) (Variables|Default|GetHealthBar) 1.0))

(event EventInteract
  (params (Actor :type Actor%20Object%20Reference))
  (bind _assassinref (Variables|Default|GetAssassinRef))
  (bind _returnvalue (Transformation|GetWorldTransform _assassinref))
  (Class|MotionWarpingComponent|AddorUpdateWarpTarget (Actor|GetComponentbyClass Actor "/Script/MotionWarping.MotionWarpingComponent") (Utilities|Struct|MakeMotionWarpingTarget (Utilities|Name|MakeLiteralName "StartAssasination") (.location _returnvalue) (Math|Rotator|MakeRotator 0.0 0.0 (+ (.yaw (.rotation _returnvalue)) 9e+01)) 0 "None" false))
  (bind _notifyname (Animation|Montage|PlayMontage (Actor|GetComponentbyClass Actor "/Script/Engine.SkeletalMeshComponent") "/Game/Characters/Mannequins/Animations/Assassinations/AM_Paired_Knife_Stealth_KidneyAndNeck_Att.AM_Paired_Knife_Stealth_KidneyAndNeck_Att")
    (:then
      (Animation|PlayAnimMontage "/Game/Characters/Mannequins/Animations/Assassinations/AM_Paired_Knife_Stealth_KidneyAndNeck_Vic.AM_Paired_Knife_Stealth_KidneyAndNeck_Vic" 1.0 "None"))
    (:OnNotifyBegin
      (if (== _notifyname "Stab")
        (Game|Damage|ApplyDamage self 25.0 0 0)
        (elif (== _notifyname "Kill")
          (Game|Damage|ApplyDamage self 1e+03 0 0))))))

(fn ConstructionScript
  (Utilities|FlowControl|Sequence
    (:then_0
      (bind _returnvalue (Rendering|Material|CreateDynamicMaterialInstance "/Game/Characters/Mannequins/Materials/Instances/Manny/MI_Manny_01.MI_Manny_01" "None" "None" :!class /Script/Engine.KismetMaterialLibrary))
      (bind _output_get (LocalVariables|SetMat01 _returnvalue))
      (Rendering|Material|SetVectorParameterValue _output_get "Tint" "(R=1.000000,G=1.000000,B=0.000000,A=1.000000)" :!class /Script/Engine.MaterialInstanceDynamic)
      (Rendering|Material|SetMaterial (Variables|Character|GetMesh) 0 (LocalVariables|GetMat01)))
    (:then_1
      (bind _returnvalue_2 (Rendering|Material|CreateDynamicMaterialInstance "/Game/Characters/Mannequins/Materials/Instances/Manny/MI_Manny_02.MI_Manny_02" "None" "None" :!class /Script/Engine.KismetMaterialLibrary))
      (bind _output_get_2 (LocalVariables|SetMat02 _returnvalue_2))
      (Rendering|Material|SetVectorParameterValue _output_get_2 "Tint" "(R=1.000000,G=1.000000,B=0.000000,A=1.000000)" :!class /Script/Engine.MaterialInstanceDynamic)
      (Rendering|Material|SetMaterial (Variables|Character|GetMesh) 1 (LocalVariables|GetMat02)))))

(fn GetActionText
  (return "Assassinate"))