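; Player character with parkour traversal, crouching, lightning attacks and stealth assassinations, which reloads ThirdPersonMap when destroyed.
; Moving into obstacles runs line traces for ledge height, thickness and clearance to choose climb or vault montages; ledge edges trigger auto-jumps.
; V runs a separate sphere-traced, motion-warped vault, and E warps into paired assassinations through BPI_Assassination.
; Montage-driven attacks combine Niagara lightning with trace damage; getters expose state and traced hand-IK points.
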(event OnComponentBeginOverlap(ObstacleCollision)
  (params (OverlappedComponent :type Primitive%20Component%20Object%20Reference) (OtherActor :type Actor%20Object%20Reference) (OtherComp :type Primitive%20Component%20Object%20Reference) (OtherBodyIndex :type Integer) (bFromSweep :type Boolean) (SweepResult :type Hit%20Result%20Structure%20%28by%20ref%29))
  (Development|PrintString (Utilities|GetDisplayName OtherComp) true true "(R=0.000000,G=0.660000,B=1.000000,A=1.000000)" 2e+01)
  (Variables|Climbing|SetInFrontOfObstacle? true))

(event OnComponentEndOverlap(ObstacleCollision)
  (params (OverlappedComponent :type Primitive%20Component%20Object%20Reference) (OtherActor :type Actor%20Object%20Reference) (OtherComp :type Primitive%20Component%20Object%20Reference) (OtherBodyIndex :type Integer))
  (Variables|Climbing|SetInFrontOfObstacle? false))

(event OnComponentEndOverlap(Box)
  (params (OverlappedComponent :type Primitive%20Component%20Object%20Reference) (OtherActor :type Actor%20Object%20Reference) (OtherComp :type Primitive%20Component%20Object%20Reference) (OtherBodyIndex :type Integer))
  ;[1 1 1] Auto Jump on Ledges
  (if (not (AI|Components|NavMovement|IsFalling (Variables|Character|GetCharacterMovement)))
    (if (> (Math|Vector|VectorLength (Variables|/Script/Engine.MovementComponent|GetVelocity (Variables|Character|GetCharacterMovement))) 4.5e+02)
      (Character|Jump))))

(event Custom|VaultMotionWarp
  (if (Variables|Default|GetCanWarp?)
    (Variables|Default|SetVaulting? true)
    (Pawn|Components|CharacterMovement|SetMovementMode (Variables|Character|GetCharacterMovement) "MOVE_Flying" 0)
    (Collision|SetActorEnableCollision false)
    (Class|MotionWarpingComponent|AddorUpdateWarpTarget (Variables|Default|GetMotionWarping) (Utilities|Struct|MakeMotionWarpingTarget (Utilities|Name|MakeLiteralName "VaultStart") (Variables|Vaulting|GetVaultStartPosition) (Transformation|GetActorRotation) 0 "None" false))
    (Class|MotionWarpingComponent|AddorUpdateWarpTarget (Variables|Default|GetMotionWarping) (Utilities|Struct|MakeMotionWarpingTarget (Utilities|Name|MakeLiteralName "VaultMiddle") (Variables|Vaulting|GetVaultMiddlePosition) (Transformation|GetActorRotation) 0 "None" false))
    (Animation|Montage|PlayMontage (Variables|Character|GetMesh) "/Game/Characters/Mannequins/Animations/Vault/AM_VaultOver.AM_VaultOver"
      (:OnCompleted
        (Pawn|Components|CharacterMovement|SetMovementMode (Variables|Character|GetCharacterMovement) "MOVE_Walking" 0)
        (Collision|SetActorEnableCollision true)
        (Variables|Default|SetVaulting? false)
        (Variables|Default|SetCanWarp? false)
        (Variables|Vaulting|SetVaultEndPosition "0.000000,0.000000,20000.000000")))))

(event Input|EnhancedActionEvents|EnhancedInputActionIA_StrongAttack
  (params (ActionValue :type Boolean) (ElapsedSeconds :type Float%20%28double-precision%29) (TriggeredSeconds :type Float%20%28double-precision%29) (InputAction :type Input%20Action%20Object%20Reference :default "/Game/Input/Actions/IA_StrongAttack.IA_StrongAttack"))
  ;[1 1 1] Attack
  (:Started
    (if (not (Variables|Default|GetAttacking?))
      (Variables|Default|SetAttacking? true)
      (Animation|Montage|PlayMontage (Variables|Character|GetMesh) "/Game/Characters/Mannequins/Animations/Magic/AM_Magic_StrongAttack_Lightning.AM_Magic_StrongAttack_Lightning" 1.0 0.0 "StartCastLightningSpell"
        (:then
          (Variables|Default|SetTempMultiplier 2.0))
        (:OnCompleted
          (Variables|Default|SetAttacking? false :!label _label))
        (:OnInterrupted
          (goto _label))))))

(event Input|EnhancedActionEvents|EnhancedInputActionIA_Move
  (params (ActionValue :type Vector%202D%20Structure) (ElapsedSeconds :type Float%20%28double-precision%29) (TriggeredSeconds :type Float%20%28double-precision%29) (InputAction :type Input%20Action%20Object%20Reference :default "/Game/Input/Actions/IA_Move.IA_Move"))
  (bind _returnvalue (Transformation|GetActorRotation))
  (bind _ledgeheight (Variables|Climbing|GetLedgeHeight))
  (bind _wallhitnormal (Variables|Climbing|GetWallHitNormal))
  (bind _returnvalue_2 (Math|Rotator|MakeRotfromX _wallhitnormal))
  (bind _returnvalue_3 (Math|Vector|GetForwardVector _returnvalue_2))
  (bind _returnvalue_4 (* _returnvalue_3 137.0))
  (bind _returnvalue_5 (+ _ledgeheight _returnvalue_4))
  (bind (_x _y _z) (Math|Vector|BreakVector _returnvalue_5))
  (bind _returnvalue_6 (+ _z -25.0))
  (bind _returnvalue_7 (Math|Vector|MakeVector _x _y _returnvalue_6))
  (:Triggered
    (if (Variables|Climbing|GetInFrontOfObstacle?)
      (if (not (Variables|Climbing|GetIsClimbing?))
        (|SetWallLocationAndNormal)
        (|SetLedgeHeight)
        (Variables|Climbing|SetJumpClearance (.z (- (Variables|Climbing|GetLedgeHeight) (Variables|Climbing|GetWallHitLocation))))
        (Variables|Climbing|SetShouldClimb? (> (Variables|Climbing|GetJumpClearance) 6e+01))
        (|TestWallThickness
          (:OutputPin
            (if (Variables|Climbing|GetShouldClimb?)
              ;[1 1 1] Climbing up/down
              (|CheckForClearance
                (:OutputPin
                  (if (Variables|Climbing|GetCanClimb?)
                    (Variables|Climbing|SetIsClimbing? true)
                    (Input|DisableInput (Game|GetPlayerController 0))
                    (|PlayClimbingAnimation)
                    (if (Variables|Climbing|GetIsWallThick?)
                      (Collision|SetCollisionEnabled (Variables|Default|GetCapsuleComponent) "QueryAndPhysics")
                      (Pawn|Components|CharacterMovement|SetMovementMode (Variables|Character|GetCharacterMovement) "MOVE_Walking" 0)
                      (Variables|Climbing|SetIsClimbing? false)
                      (Input|EnableInput (Game|GetPlayerController 0))
                      (else
                        (Animation|PlayAnimMontage "/Game/Characters/Mannequins/Animations/Parkour/MQ_JumpingDownFromWall_RM_Montage.MQ_JumpingDownFromWall_RM_Montage" 1.0 "StartJumpDown")
                        (Utilities|FlowControl|Delay 1.63)
                        (Collision|SetCollisionEnabled (Variables|Default|GetCapsuleComponent) "QueryAndPhysics")
                        (Pawn|Components|CharacterMovement|SetMovementMode (Variables|Character|GetCharacterMovement) "MOVE_Walking" 0)
                        (Variables|Climbing|SetIsClimbing? false)
                        (Input|EnableInput (Game|GetPlayerController 0)))))))
              (else
                ;[1 1 1] Vaulting
                (Variables|Climbing|SetIsClimbing? true)
                (Input|DisableInput (Game|GetPlayerController 0))
                (Pawn|Components|CharacterMovement|DisableMovement (Variables|Character|GetCharacterMovement))
                (Collision|SetCollisionEnabled (Variables|Default|GetCapsuleComponent) "NoCollision")
                (Pawn|Components|CharacterMovement|SetMovementMode (Variables|Character|GetCharacterMovement) "MOVE_Flying" 0)
                (Transformation|SetActorRotation (Math|Rotator|MakeRotator (.roll _returnvalue) (.pitch _returnvalue) (+ (.yaw (Math|Rotator|MakeRotfromX (Variables|Climbing|GetWallHitNormal))) 1.8e+02)))
                (Transformation|SetActorLocation _returnvalue_7 false false)
                (Rendering|Debug|DrawDebugBox _returnvalue_7 "1.000000,1.000000,1.000000" "(R=1.000000,G=0.000000,B=0.000000,A=1.000000)" "0, 0, 0" 2e+01 0.0)
                (if (Variables|Climbing|GetIsWallThick?)
                  (bind _returnvalue_8 (Animation|PlayAnimMontage "/Game/Characters/Mannequins/Animations/Parkour/MQ_GettingUp_RM_Montage.MQ_GettingUp_RM_Montage" 1.0 "None"))
                  (Utilities|FlowControl|Delay _returnvalue_8)
                  (else
                    (bind _returnvalue_9 (Animation|PlayAnimMontage "/Game/Characters/Mannequins/Animations/Parkour/MQ_Vault_RM_Montage.MQ_Vault_RM_Montage" 1.0 "None"))
                    (Utilities|FlowControl|Delay _returnvalue_9)))
                (Collision|SetCollisionEnabled (Variables|Default|GetCapsuleComponent) "QueryAndPhysics")
                (Pawn|Components|CharacterMovement|SetMovementMode (Variables|Character|GetCharacterMovement) "MOVE_Walking" 0)
                (Variables|Climbing|SetIsClimbing? false)
                (Input|EnableInput (Game|GetPlayerController 0))))))))))

(event Input|EnhancedActionEvents|EnhancedInputActionIA_Interact
  (params (ActionValue :type Boolean) (ElapsedSeconds :type Float%20%28double-precision%29) (TriggeredSeconds :type Float%20%28double-precision%29) (InputAction :type Input%20Action%20Object%20Reference :default "/Game/Input/Actions/IA_Interact.IA_Interact"))
  ;[1 1 1] Attack
  (:Started
    (if (not (Variables|Default|GetAttacking?))
      (Variables|Default|SetAttacking? true)
      (Animation|Montage|PlayMontage (Variables|Character|GetMesh) "/Game/Characters/Mannequins/Animations/Magic/AM_Magic_QuickAttack_Lightning.AM_Magic_QuickAttack_Lightning" 1.0 0.0 "StartCastLightningSpell"
        (:then
          (Variables|Default|SetTempMultiplier 1.0))
        (:OnCompleted
          (Variables|Default|SetAttacking? false :!label _label))
        (:OnInterrupted
          (goto _label))))))

(event Input|EnhancedActionEvents|EnhancedInputActionIA_Crouch
  (params (ActionValue :type Boolean) (ElapsedSeconds :type Float%20%28double-precision%29) (TriggeredSeconds :type Float%20%28double-precision%29) (InputAction :type Input%20Action%20Object%20Reference :default "/Game/Input/Actions/IA_Crouch.IA_Crouch"))
  ;[1 1 1] Crouching
  (:Started
    (if (AI|Components|NavMovement|IsCrouching (Variables|Character|GetCharacterMovement))
      (Character|UnCrouch)
      (else
        (Character|Crouch)))))

(event EventEndHandIK
  (Variables|IK|SetUseHandIK? false)
  (Development|PrintString "Not Using Hand IK"))

(event EventDestroyed
  (Game|OpenLevel(byName) "ThirdPersonMap"))

(event EventStartHandIK
  (Variables|IK|SetUseHandIK? true)
  (Development|PrintString "Using Hand IK"))

(event EventShootLightning
  (bind _ns_lightning (Variables|Default|GetNS_Lightning))
  (bind _mesh (Variables|Character|GetMesh))
  (bind _returnvalue (Transformation|GetSocketLocation _mesh "MagicSocket_Right"))
  ;[1 1 1] Lightning Attack
  (Effects|Components|ParticleSystem|SetVectorParameter _ns_lightning "LightningOrigin" (Math|Transform|InverseTransformLocation (Transformation|GetActorTransform) (Transformation|GetSocketLocation (Variables|Character|GetMesh) "MagicSocket_Right")))
  (Effects|Components|ParticleSystem|SetVectorParameter _ns_lightning "LightningTarget" "1000.000000,0.000000,0.000000")
  (Components|Activation|Activate _ns_lightning true)
  (bind (_outhit _returnvalue_2) (Class|KismetSystemLibrary|SphereTraceSinglebyProfile _returnvalue (+ _returnvalue (* (Math|Vector|GetForwardVector (Transformation|GetActorRotation)) 1e+03)) 0.0 "Enemy" false 0 "ForDuration" true))
  (if _returnvalue_2
    (Game|Damage|ApplyDamage (.HitActor (Collision|BreakHitResult _outhit)) (* 5e+01 (Variables|Default|GetTempMultiplier)) 0 self)))

(event EventChargeLightning
  (bind _ns_lightning (Variables|Default|GetNS_Lightning))
  ;[1 1 1] Lightning Attack
  (Effects|Components|ParticleSystem|SetVectorParameter _ns_lightning "LightningOrigin" "0.000000,0.000000,1000.000000")
  (Effects|Components|ParticleSystem|SetVectorParameter _ns_lightning "LightningTarget" (Math|Transform|InverseTransformLocation (Transformation|GetActorTransform) (Transformation|GetSocketLocation (Variables|Character|GetMesh) "MagicSocket_Right")))
  (Components|Activation|Activate _ns_lightning true))

(event Input|KeyboardEvents|V
  (params (Key :type Key%20Structure :default "None"))
  (:Pressed
    (CallFunction|Vault)))

(event Input|KeyboardEvents|E
  (params (Key :type Key%20Structure :default "None"))
  (:Pressed
    (bind _array_element (Utilities|Array|ForEachLoopwithBreak (Class|Actor|GetOverlappingComponents) :!label _label)
      (:LoopBody
        (Utilities|IsValid _array_element
          (:Is%20Valid
            (Variables|Default|SetAssassinationTarget (Components|GetOwner _array_element))
            (if (Utilities|DoesObjectImplementInterface (Components|GetOwner _array_element) "/Game/Blueprints/Dummy/BPI_Assassination.BPI_Assassination_C")
              (goto _label Break)))))
      (:Completed
        (bind _assassinationtarget (Variables|Default|GetAssassinationTarget)
          (:then
            (bind (_referencelocation _referencerotation) (Class|BPIAssassination|StealthBackAssassin(Message) _assassinationtarget))
            (Variables|Default|SetAssassinationTarget 0)
            (Class|MotionWarpingComponent|AddorUpdateWarpTarget (Variables|Default|GetMotionWarping) (Utilities|Struct|MakeMotionWarpingTarget (Utilities|Name|MakeLiteralName "StartAssasination") _referencelocation _referencerotation 0 "None" false))
            (bind _notifyname (Animation|Montage|PlayMontage (Variables|Character|GetMesh) "/Game/Characters/Mannequins/Animations/Assassinations/AM_Paired_Knife_Stealth_KidneyAndNeck_Att.AM_Paired_Knife_Stealth_KidneyAndNeck_Att")
              (:OnNotifyBegin
                (if (== _notifyname "Stab")
                  (Game|Damage|ApplyDamage (Variables|Default|GetAssassinationTarget) 25.0 0 0)
                  (elif (== _notifyname "Kill")
                    (Game|Damage|ApplyDamage (Variables|Default|GetAssassinationTarget) 1e+03 0 0))))))
          (:else))))))

(fn ConstructionScript
  (Utilities|FlowControl|Sequence
    (:then_0
      (bind _returnvalue (Rendering|Material|CreateDynamicMaterialInstance "/Game/Characters/Mannequins/Materials/Instances/Manny/MI_Manny_01.MI_Manny_01" "None" "None" :!class /Script/Engine.KismetMaterialLibrary))
      (bind _output_get (LocalVariables|SetMat01 _returnvalue))
      (Rendering|Material|SetVectorParameterValue _output_get "Tint" "(R=0.000000,G=0.000000,B=0.000000,A=1.000000)" :!class /Script/Engine.MaterialInstanceDynamic)
      (Rendering|Material|SetMaterial (Variables|Character|GetMesh) 0 (LocalVariables|GetMat01)))
    (:then_1
      (bind _returnvalue_2 (Rendering|Material|CreateDynamicMaterialInstance "/Game/Characters/Mannequins/Materials/Instances/Manny/MI_Manny_02.MI_Manny_02" "None" "None" :!class /Script/Engine.KismetMaterialLibrary))
      (bind _output_get_2 (LocalVariables|SetMat02 _returnvalue_2))
      (Rendering|Material|SetVectorParameterValue _output_get_2 "Tint" "(R=0.000000,G=0.000000,B=0.000000,A=1.000000)" :!class /Script/Engine.MaterialInstanceDynamic)
      (Rendering|Material|SetMaterial (Variables|Character|GetMesh) 1 (LocalVariables|GetMat02)))))

(fn LedgeHandIKBoth
  (Utilities|FlowControl|Sequence
    (:then_0
      (bind _handvector (CallFunction|LedgeHandIKSingle "VB clavicle_l_hand_l"))
      (Variables|IK|SetLeftHandIKVector _handvector))
    (:then_1
      (bind _handvector_2 (CallFunction|LedgeHandIKSingle "VB clavicle_r_hand_r"))
      (Variables|IK|SetRightHandIKVector _handvector_2))))

(fn LedgeHandIKSingle
  (params (SocketName :type Name))
  (bind _mesh (Variables|Character|GetMesh))
  (bind _returnvalue (Transformation|GetSocketLocation _mesh SocketName))
  (bind (_outhit _returnvalue_2) (Collision|SphereTraceByChannel _returnvalue (+ _returnvalue (* (Math|Vector|GetUpVector (Transformation|GetActorRotation)) -6e+01)) 1e+01 "TraceTypeQuery1" false 0 (Variables|Climbing|GetClimbing%20Debug) true "(R=0.000000,G=0.000000,B=0.000000,A=1.000000)"))
  (if _returnvalue_2
    (bind (_outhit_2 _returnvalue_3) (Collision|SphereTraceByChannel (+ (.Location (Collision|BreakHitResult _outhit)) "0.000000,0.000000,20.000000") (- (.Location (Collision|BreakHitResult _outhit)) "0.000000,0.000000,10.000000") 1e+01 "TraceTypeQuery1" false 0 (Variables|Climbing|GetClimbing%20Debug)))
    (if _returnvalue_3
      (return (Math|Vector|MakeVector (.x (+ (.ImpactPoint (Collision|BreakHitResult _outhit)) (* (Math|Vector|GetForwardVector (Math|Rotator|MakeRotfromX (.ImpactNormal (Collision|BreakHitResult _outhit)))) 5.0))) (.y (+ (.ImpactPoint (Collision|BreakHitResult _outhit)) (* (Math|Vector|GetForwardVector (Math|Rotator|MakeRotfromX (.ImpactNormal (Collision|BreakHitResult _outhit)))) 5.0))) (- (.Z (Math|Vector|BreakVector (.ImpactPoint (Collision|BreakHitResult _outhit_2)))) 1e+01))))))

(fn Vault
  (bind _index (Utilities|FlowControl|ForLoopwithBreak 0 2 :!label _label)
    (:LoopBody
      (bind (_outhit _returnvalue) (Collision|SphereTraceByChannel (+ (Transformation|GetActorLocation) (Math|Vector|MakeVector 0.0 0.0 (* _index 30))) (+ (+ (Transformation|GetActorLocation) (Math|Vector|MakeVector 0.0 0.0 (* _index 30))) (* (Math|Vector|GetForwardVector (Transformation|GetActorRotation)) 1.8e+02)) 5.0 "TraceTypeQuery1" false 0 "ForDuration"))
      (if _returnvalue
        (Utilities|FlowControl|Sequence
          (:then_0
            (goto _label Break))
          (:then_1
            (bind _index_2 (Utilities|FlowControl|ForLoopwithBreak 0 5 :!label _label_2)
              (:LoopBody
                (bind (_outhit_2 _returnvalue_2) (Collision|SphereTraceByChannel (+ (+ (.Location (Collision|BreakHitResult _outhit)) "0.000000,0.000000,100.000000") (* (Math|Vector|GetForwardVector (Transformation|GetActorRotation)) (* _index_2 50))) (- (+ (+ (.Location (Collision|BreakHitResult _outhit)) "0.000000,0.000000,100.000000") (* (Math|Vector|GetForwardVector (Transformation|GetActorRotation)) (* _index_2 50))) "0.000000,0.000000,100.000000") 1e+01 "TraceTypeQuery1" false 0 "ForDuration"))
                (if _returnvalue_2
                  (if (== _index_2 0)
                    (bind _output_get (Variables|Vaulting|SetVaultStartPosition (.Location (Collision|BreakHitResult _outhit_2))))
                    (Rendering|Debug|DrawDebugSphere _output_get 1e+01 12 "(R=1.000000,G=0.000000,B=1.000000,A=1.000000)" 1e+01 2.0)
                    (else
                      (bind _output_get_2 (Variables|Vaulting|SetVaultMiddlePosition (.Location (Collision|BreakHitResult _outhit_2))))
                      (Rendering|Debug|DrawDebugSphere _output_get_2 1e+01 12 "(R=1.000000,G=1.000000,B=0.000000,A=1.000000)" 1e+01 2.0)
                      (Variables|Default|SetCanWarp? true)))
                  (else
                    (bind (_outhit_3 _returnvalue_3) (Collision|LineTraceByChannel (+ (.TraceStart (Collision|BreakHitResult _outhit_2)) (* (Math|Vector|GetForwardVector (Transformation|GetActorRotation)) 8e+01)) (- (+ (.TraceStart (Collision|BreakHitResult _outhit_2)) (* (Math|Vector|GetForwardVector (Transformation|GetActorRotation)) 8e+01)) "0.000000,0.000000,1000.000000") "TraceTypeQuery1" false 0 "ForDuration" true "(R=0.000000,G=1.000000,B=1.000000,A=1.000000)"))
                    (if _returnvalue_3
                      (bind _output_get_3 (Variables|Vaulting|SetVaultEndPosition (.Location (Collision|BreakHitResult _outhit_3))))
                      (Utilities|FlowControl|Sequence
                        (:then_0
                          (goto _label_2 Break))
                        (:then_1
                          (Rendering|Debug|DrawDebugSphere _output_get_3 1e+01 12 "(R=0.000000,G=1.000000,B=1.000000,A=1.000000)" 2e+01 2.0)
                          (CallFunction|VaultMotionWarp))))))))))))))

(fn GetEquipmentAnimationType
  (return (Variables|Animation|GetEquipment%20Animation%20Type)))

(fn GetHandIKVectors
  (return (Variables|IK|GetLeftHandIKVector) (Variables|IK|GetRightHandIKVector)))

(fn IsAttacking
  (return (Variables|Default|GetAttacking?)))

(fn IsClimbing
  (return (Variables|Climbing|GetIsClimbing?)))

(fn IsVaulting
  (return (Variables|Default|GetVaulting?)))